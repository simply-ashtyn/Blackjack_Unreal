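; Blackjack deck component that runs the card game's rounds, dealing, scoring and dealer turn.
; It shuffles once at BeginPlay and deals by advancing an index, which NextRound never resets.
; CalculateScore reads card values from DT_DeckData, dropping Aces from 11 to 1 on a bust.
; Dispatchers announce hand and round changes; the dealer draws through 16, and results create BP_WinLose widgets, though the Blackjack one is never added to the viewport.
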(event Custom|UpdateHands
  (Default|CallOnPlayerHandUpdated))

(event EventBeginPlay
  (CallFunction|ShuffleDeck)
  (CallFunction|BeginRound))

(fn ShuffleDeck
  (Utilities|Array|Shuffle (Variables|Default|GetDeck)))

(fn Deal
  (params (Hand :type Array%20of%20Names) (Player :type Boolean))
  (bind _playerhand (Variables|Default|GetPlayerHand))
  (bind _dealerhand (Variables|Default|GetDealerHand))
  (bind _deckindex (Variables|Default|GetDeckIndex))
  (bind _deck (Variables|Default|GetDeck))
  ;[0.5051 1 0.508] Original Design - a little clunky but functional
  (if (< (Utilities|Array|Length Hand) 2)
    ;;[1 1 1] Initial Deal
    (Utilities|Array|Add Hand (Utilities|Array|Get(acopy) _deck (Variables|Default|GetDeckIndex)))
    (Math|Integer|IncrementInt _deckindex
      (:%20%20
        (Utilities|Array|Add Hand (Utilities|Array|Get(acopy) _deck _deckindex))
        (Math|Integer|IncrementInt (Variables|Default|GetDeckIndex)
          (:%20%20
            (CallFunction|UpdateHands)))))
    (else
      (if Player
        (Utilities|Array|Add _playerhand (Utilities|Array|Get(acopy) (Variables|Default|GetDeck) (Variables|Default|GetDeckIndex)))
        (bind _newscore (CallFunction|CalculateScore _playerhand))
        (bind _output_get (Variables|Default|SetPlayerScore _newscore))
        (if (> _output_get 21)
          (Variables|Default|SetbPlayerBust true))
        (Variables|Default|SetbIsPlayer false)
        (Math|Integer|IncrementInt (Variables|Default|GetDeckIndex)
          (:%20%20
            _))
        (else
          (Utilities|Array|Add _dealerhand (Utilities|Array|Get(acopy) (Variables|Default|GetDeck) (Variables|Default|GetDeckIndex)))
          (bind _newscore_2 (CallFunction|CalculateScore _dealerhand))
          (bind _output_get_2 (Variables|Default|SetDealerScore _newscore_2))
          (if (> _output_get_2 21)
            (Variables|Default|SetbDealerBust true))
          (Math|Integer|IncrementInt (Variables|Default|GetDeckIndex)
            (:%20%20
              _))))
      (CallFunction|UpdateHands))))

(fn CalculateScore
  (params (Hand :type Array%20of%20Names))
  (for _array_element Hand
    (bind _returnvalue (Utilities|GetDataTableRow "/Game/Actors/Cards/DT_DeckData.DT_DeckData" _array_element)
      (:then
        (if (== (.value _returnvalue) 11)
          (Math|Integer|IncrementInt (LocalVariables|GetAceCount)
            (:%20%20
              _)))
        (LocalVariables|SetLocalScore (+ (LocalVariables|GetLocalScore) (.value _returnvalue))))))
  (if (and (> (LocalVariables|GetLocalScore) 21) (> (LocalVariables|GetAceCount) 0))
    (while (and (> (LocalVariables|GetAceCount) 0) (> (LocalVariables|GetLocalScore) 21))
      (LocalVariables|SetLocalScore (- (LocalVariables|GetLocalScore) 10))
      (Math|Integer|DecrementInt (LocalVariables|GetAceCount)))
    (return (LocalVariables|GetLocalScore))
    (else
      (return (LocalVariables|GetLocalScore)))))

(fn DealersTurn
  (bind _self self)
  (bind _playerscore (Variables|Default|GetPlayerScore))
  (bind _dealerscore (Variables|Default|GetDealerScore))
  (bind _bplayerbust (Variables|Default|GetbPlayerBust))
  (if _bplayerbust
    (bind _returnvalue (UserInterface|CreateWidget "/Game/Widgets/BP_WinLose.BP_WinLose_C" 0 1 _self :!label _label))
    (UserInterface|Viewport|AddtoViewport _returnvalue 0)
    (else
      (while (Math|Boolean|ANDBoolean (not (Variables|Default|GetbDealerBust)) (<= (Variables|Default|GetDealerScore) 16) (not _bplayerbust))
        (CallFunction|Deal (Variables|Default|GetDealerHand) false))
      (if (or (> _playerscore _dealerscore) (Variables|Default|GetbDealerBust))
        (bind _returnvalue_2 (UserInterface|CreateWidget "/Game/Widgets/BP_WinLose.BP_WinLose_C" 0 0 _self))
        (UserInterface|Viewport|AddtoViewport _returnvalue_2 0)
        (elif (> _dealerscore _playerscore)
          (goto _label)
          (else
            (bind _returnvalue_3 (UserInterface|CreateWidget "/Game/Widgets/BP_WinLose.BP_WinLose_C" 0 -1 _self))
            (UserInterface|Viewport|AddtoViewport _returnvalue_3 0)))))))

(fn NextRound
  (Utilities|Array|Clear (Variables|Default|GetPlayerHand))
  (Utilities|Array|Clear (Variables|Default|GetDealerHand))
  (Variables|Default|SetPlayerScore 0)
  (Variables|Default|SetDealerScore 0)
  (Variables|Default|SetbDealerBust false)
  (Variables|Default|SetbPlayerBust false)
  (Variables|Default|SetbIsPlayer true)
  (Default|CallOnNewRound)
  (CallFunction|BeginRound))

(fn BeginRound
  ;[1 1 1] Original version
  (CallFunction|Deal (Variables|Default|GetPlayerHand) true)
  (CallFunction|Deal (Variables|Default|GetDealerHand) false)
  (bind _newscore (CallFunction|CalculateScore (Variables|Default|GetPlayerHand)))
  (Variables|Default|SetPlayerScore _newscore)
  (bind _newscore_2 (CallFunction|CalculateScore (Variables|Default|GetDealerHand)))
  (Variables|Default|SetDealerScore _newscore_2)
  (CallFunction|UpdateHands)
  (if (or (== (Variables|Default|GetPlayerScore) 21) (== (Variables|Default|GetDealerScore) 21))
    (Variables|Default|SetbBlackjack true)
    (if (== (Variables|Default|GetDealerScore) 21)
      (LocalVariables|SetWinner 1)
      (else
        (LocalVariables|SetWinner 0)))
    (CallFunction|Blackjack (LocalVariables|GetWinner))))

(fn Blackjack
  (params (WinnderEnum :type Integer))
  (bind _returnvalue (UserInterface|CreateWidget "/Game/Widgets/BP_WinLose.BP_WinLose_C" 0 WinnderEnum self (Variables|Default|GetbBlackjack)))
  (Widget|SetFocus _returnvalue))